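; Homing missile actor that seeks enemies, deals fixed damage to an AEnemy it hits, and destroys itself on any hit.
; From BeginPlay it re-runs LockOn on a short repeating delay, feeding the found target's scene component to ProjectileMovement as the homing target.
; The search scans EnemyCharacter actors tagged "Homing", snapping rotation toward each closer candidate.
; ClosestDistance is not reset between searches.
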(event `self.ReceiveHit`
  (params (MyComp :type "PrimitiveComponent Object Reference") (Other :type "Actor Object Reference") (OtherComp :type "PrimitiveComponent Object Reference") (bSelfMoved :type Boolean) (HitLocation :type "Vector Structure") (HitNormal :type "Vector Structure") (NormalImpulse :type "Vector Structure") (Hit :type "HitResult Structure (by ref)"))
  (bind _asaenemy (cast `AEnemy` Other)
    (:`then`
      (`AEnemy.OnTakeDamage` _asaenemy 20.0))
    (:`CastFailed`
      _))
  (`self.K2_DestroyActor`))

(event `LockOn`
  (bind _projectilemovement (`self.ProjectileMovement`))
  (bind _target (`self.findClosestHomingTarget`))
  (set `ProjectileMovementComponent.HomingTargetComponent` _target _projectilemovement)
  (set `ProjectileMovementComponent.bIsHomingProjectile` true _projectilemovement))

(event `self.ReceiveBeginPlay`
  (set `ProjectileMovementComponent.InitialSpeed` 200.0 (`self.ProjectileMovement`))
  (`self.LockOn` :!label _label)
  (`KismetSystemLibrary.Delay` 0.2)
  (goto _label))

(fn `findClosestHomingTarget`
  (returns (target :type "SceneComponent Object Reference"))
  (bind _returnvalue (`self.K2_GetActorLocation`))
  (bind _returnvalue_2 (`self.GetComponentByClass` (`self.CurrentTarget`) "/Script/Engine.SceneComponent"))
  (bind _outactors (`GameplayStatics.GetAllActorsOfClassWithTag` "/Game/Game/Blueprint/EnemyCharacter.EnemyCharacter_C" "Homing"))
  (for _array_element _outactors
    (bind _returnvalue_3 (`self.K2_GetActorLocation` _array_element))
    (bind _returnvalue_4 (`KismetMathLibrary.VSize` (- _returnvalue_3 _returnvalue)))
    (if (< _returnvalue_4 (`self.Closest Distance`))
      (set `self.Closest Distance` _returnvalue_4)
      (set `self.CurrentTarget` _array_element)
      (`self.K2_SetActorRotation` (`KismetMathLibrary.FindLookAtRotation` _returnvalue _returnvalue_3))))
  (if (not (== _returnvalue_2 null))
    (return _returnvalue_2)))

(fn `UserConstructionScript`)