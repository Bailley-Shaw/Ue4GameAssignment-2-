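; BP_MainCharacter is the main character Blueprint, handling the UI for character prompts, quests and inventory.
; BeginPlay creates the quest and inventory widgets, hides the inventory and sets game-only input.
; Events create or dismiss the player UI on demand and forward quest info, completion messages and quest list updates to the widgets.
; The inventory refresh event shows that widget and rebuilds it from EquipmentInventory.
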(event `self.OnShowUI`
  (params (Character :type Name))
  ;[1 1 1] Showing and hiding ui
  (if (not (`KismetSystemLibrary.IsValid` (`self.PlayerUI`)))
    (bind _returnvalue (`|CreateWidget` "/Game/Game/UI/WBP_PlayerUI.WBP_PlayerUI_C" (`GameplayStatics.GetPlayerController` 0)))
    (`UserWidget.AddToViewport` _returnvalue 0)
    (bind _output_get (set `self.PlayerUI` _returnvalue))
    (`/Game/Game/UI/WBP_PlayerUI.ShowUI` _output_get (`KismetTextLibrary.Conv_NameToText` Character))))

(event `self.OnHideUI`
  (bind _playerui (`self.PlayerUI`))
  ;[1 1 1] Showing and hiding ui
  (if (`KismetSystemLibrary.IsValid` _playerui)
    (`UINavWidget.ReturnToParent` _playerui false 0)
    (set `self.PlayerUI` null)))

(event `self.ReceiveBeginPlay`
  (bind _returnvalue (`GameplayStatics.GetPlayerController` 0))
  ;[1 1 1] Initialization - done through blueprints for ui related things
  (bind _returnvalue_2 (`|CreateWidget` "/Game/Game/UI/Quest/WBP_Quest.WBP_Quest_C" _returnvalue))
  (`UserWidget.AddToViewport` _returnvalue_2 0)
  (set `self.QuestUI` _returnvalue_2)
  (bind _returnvalue_3 (`|CreateWidget` "/Game/Game/UI/Inventory/WBP_Inventory.WBP_Inventory_C"))
  (bind _output_get (set `self.InventoryUI` _returnvalue_3))
  (`UserWidget.AddToViewport` _output_get 0)
  (`/Game/Game/UI/Inventory/WBP_Inventory.Hide` _output_get)
  (`WidgetBlueprintLibrary.SetInputMode_GameOnly` _returnvalue))

(event `self.OnRefreshInventory`
  (bind _inventoryui (`self.InventoryUI`))
  ;[1 1 1] OnRefreshInventory - again refreshes ui
  (if (`KismetSystemLibrary.IsValid` _inventoryui)
    (`/Game/Game/UI/Inventory/WBP_Inventory.Show` _inventoryui)
    (`/Game/Game/UI/Inventory/WBP_Inventory.Refresh Inventory` _inventoryui (`self.EquipmentInventory`))))

(event `self.OnShowUpdatedQuestList`
  (params (QuestTextList :type "Array of Text (by ref)"))
  (bind _questui (`self.QuestUI`))
  ;[1 1 1] ui wuests sytem
  (if (`KismetSystemLibrary.IsValid` _questui)
    (`/Game/Game/UI/Quest/WBP_Quest.UpdateQuestList` _questui QuestTextList)))

(event `self.OnShowQuestInfo`
  (params (Quest :type "Quest Structure"))
  (bind _playerui (`self.PlayerUI`))
  ;[1 1 1] ui wuests sytem
  (if (`KismetSystemLibrary.IsValid` _playerui)
    (`/Game/Game/UI/WBP_PlayerUI.ShowQuestInfo` _playerui Quest_Message Quest_ItemQuestTexture)))

(event `self.OnShowQuestCompleted`
  (params (Message :type "Text (by ref)"))
  (bind _playerui (`self.PlayerUI`))
  ;[1 1 1] ui wuests sytem
  (if (`KismetSystemLibrary.IsValid` _playerui)
    (`/Game/Game/UI/WBP_PlayerUI.ShowQuestCompleted` _playerui Message)))

(fn `UserConstructionScript`)