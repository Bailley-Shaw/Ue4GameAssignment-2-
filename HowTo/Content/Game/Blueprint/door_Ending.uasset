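; Ending door actor that finishes the game with an ending screen when its reward event fires.
; OnPlayerEnter plays a balloon sound at the door.
; OnReward rotates the mesh a single lerp step toward a yaw or roll target, shows the Ending widget, plays a crash sound and switches the player controller to UI-only input.
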(event `self.OnPlayerEnter`
  (`GameplayStatics.SpawnSoundAtLocation` "/Game/Game/SFX/Balloon_003.Balloon_003" (`self.K2_GetActorLocation`) (struct) 1.0 1.0 0.0 null null))

(event `self.onReward`
  (bind _returnvalue (`GameplayStatics.GetPlayerController` 0))
  (bind _staticmesh (`self.StaticMesh`))
  (`SceneComponent.K2_SetWorldRotation` _staticmesh (`KismetMathLibrary.RLerp` (`SceneComponent.K2_GetComponentRotation` _staticmesh) (struct :`Yaw` -180.0) 0.1) false false)
  (bind _returnvalue_2 (`|CreateWidget` "/Game/Game/UI/MainMenu/Ending.Ending_C" _returnvalue))
  (`UserWidget.AddToViewport` _returnvalue_2 0)
  (`GameplayStatics.PlaySoundAtLocation` "/Game/Game/136629__smmassuda__crashing.136629__smmassuda__crashing" (`self.K2_GetActorLocation`) (struct) 1.0 1.0 0.0 null null null)
  (`WidgetBlueprintLibrary.SetInputMode_UIOnlyEx` _returnvalue null))

(fn `UserConstructionScript`)