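; BP_MainGameMode is a game mode that plays a 2D sound on BeginPlay and keeps enemies spawning around the player.
; A fast looping timer counts EnemyCharacter actors and spawns one whenever fewer than three exist.
; Each spawn location is a random navigable point within a very small radius of the player character's location, so placement relies on navigation data.
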(event `self.ReceiveBeginPlay`
  (`GameplayStatics.PlaySound2D` null 1.0 1.0 0.0 null null)
  (`KismetSystemLibrary.K2_SetTimerDelegate` (delegate `spawnEnemies`) 0.2 true))

(event `spawnEnemies`
  (bind _outactors (`GameplayStatics.GetAllActorsOfClass` "/Game/Game/Blueprint/EnemyCharacter.EnemyCharacter_C"))
  (if (not (>= (`KismetArrayLibrary.Array_Length` _outactors) 3))
    (`|SpawnActorFromClass` "/Game/Game/Blueprint/EnemyCharacter.EnemyCharacter_C" (`KismetMathLibrary.MakeTransform` (`NavigationSystemV1.K2_GetRandomLocationInNavigableRadius` (`self.K2_GetActorLocation` (`GameplayStatics.GetPlayerCharacter` 0)) 10.0 null null)) "Undefined" "OverrideRootScale" null null)))

(fn `UserConstructionScript`)